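; BP_SlidingDoor is an interactable door that slides open in response to an event from BP_Bomb.
; On BeginPlay it finds a BP_Bomb in the level with GetActorOfClass and binds its Open event to that bomb's OpenDoor dispatcher.
; Open plays a timeline that lerps the Door's relative location from start to end, with no sweep and no closing logic.
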(event Custom|Open
  (bind _alpha (Timeline|Timeline Play)
    (:Update
      (Transformation|SetRelativeLocation (Variables|Default|GetDoor) (Math|Vector|Lerp(Vector) (Variables|Default|GetDoorStartLocation) (Variables|Default|GetDoorEndLocation) _alpha) false false))))

(event EventBeginPlay
  (Utilities|FlowControl|Sequence
    (:then_0
      (bind _returnvalue (Actor|GetActorOfClass "/Game/Interactables/BP_Bomb.BP_Bomb_C"))
      (Variables|Default|SetBombREF _returnvalue))
    (:then_1
      (EventDispatchers|BindEventtoOpenDoor (Variables|Default|GetBombREF) (delegate Custom|Open)))))

(fn ConstructionScript)