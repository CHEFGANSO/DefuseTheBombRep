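; BP_Bomb is an interactable bomb that the player defuses through a keypad widget.
; On BeginPlay it creates UI_Keypad, caches the game mode and binds the widget's success and failure events.
; Interacting shows the keypad in UI-only input; either result closes it and restores game input.
; Success also turns the light green, blocks further Visibility traces on the cube, stops the game mode countdown and calls OpenDoor.
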(event Custom|Failure
  (bind _returnvalue (Game|GetPlayerController 0))
  (Widget|RemovefromParent (Variables|Default|GetUI_Keypad))
  (Variables|/Script/Engine.PlayerController|SetbShowMouseCursor _returnvalue false)
  (Input|SetInputModeGameOnly _returnvalue false))

(event Custom|Defuse
  (bind _returnvalue (Game|GetPlayerController 0))
  (Widget|RemovefromParent (Variables|Default|GetUI_Keypad))
  (Variables|/Script/Engine.PlayerController|SetbShowMouseCursor _returnvalue false)
  (Input|SetInputModeGameOnly _returnvalue false)
  (Rendering|Components|Light|SetLightColor (Variables|Default|GetPointLight) "(R=0.000000,G=1.000000,B=0.000000,A=1.000000)" true)
  (Collision|SetCollisionResponsetoChannel (Variables|Default|GetCube) "ECC_Visibility" "ECR_Ignore")
  (Variables|/Game/FirstPerson/Blueprints/BP_FirstPersonGameMode.BP_FirstPersonGameMode_C|SetCountdown? (Variables|Default|GetGameModeREF) false)
  (Default|CallOpenDoor))

(event EventInteract
  (UserInterface|Viewport|AddtoViewport (Variables|Default|GetUI_Keypad) 0)
  (Variables|/Script/Engine.PlayerController|SetbShowMouseCursor (Game|GetPlayerController 0) true)
  (Input|SetInputModeUIOnly (Game|GetPlayerController 0) (Variables|Default|GetUI_Keypad) "DoNotLock" false))

(event EventBeginPlay
  (Utilities|FlowControl|Sequence
    (:then_0
      (bind _returnvalue (UserInterface|CreateWidget "/Game/Interactables/UI/UI_Keypad.UI_Keypad_C"))
      (Variables|Default|SetUI_Keypad _returnvalue))
    (:then_1
      (bind _asbp_first_person_game_mode (Utilities|Casting|CastToBP_FirstPersonGameMode (Game|GetGameMode)))
      (Variables|Default|SetGameModeREF _asbp_first_person_game_mode))
    (:then_2
      (EventDispatchers|BindEventtoSuccess! (Variables|Default|GetUI_Keypad) (delegate Custom|Defuse)))
    (:then_3
      (EventDispatchers|BindEventtoFailure! (Variables|Default|GetUI_Keypad) (delegate Custom|Failure)))))

(fn ConstructionScript
  (|CallParentFunction))