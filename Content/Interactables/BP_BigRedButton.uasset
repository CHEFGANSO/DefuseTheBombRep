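; Big red button interactable that runs a reaction-timing minigame: press it while its light flashes yellow to win.
; While the player's hover flag is set, Tick opens the cover and starts a looping timer with a random interval; losing hover reverses both.
; Each timer firing briefly makes the button winnable.
; Interact animates the press, and a win keeps the timer cleared and the light yellow.
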(event Custom|GameLogic
  (Variables|Default|SetIsButtonReady? true)
  (Rendering|Material|SetMaterial (Variables|Default|GetLight) 0 "/Game/Interactables/StaticMeshes/Materials/M_Yellow_Plastic.M_Yellow_Plastic")
  (Utilities|FlowControl|Delay 0.4)
  (Variables|Default|SetIsButtonReady? false)
  (Rendering|Material|SetMaterial (Variables|Default|GetLight) 0 "/Game/Interactables/StaticMeshes/Materials/M_Red_Plastic.M_Red_Plastic"))

(event Custom|StartGame
  (Utilities|FlowControl|DoOnce false
    (:Completed
      (bind _returnvalue (Utilities|Time|SetTimerbyEvent (delegate Custom|GameLogic) (Math|Random|RandomFloatinRange 2.0 5.0) true)))))

(event Custom|EndGame
  (Utilities|Time|ClearandInvalidateTimerbyHandle (stale Custom|StartGame _returnvalue))
  (Variables|Default|SetIsButtonReady? false)
  (Utilities|FlowControl|DoOnce false) ; enters at Reset
)

(event EventInteract
  (if (Variables|Default|GetIsButtonReady?)
    (Variables|Default|SetWin? true))
  (Utilities|FlowControl|DoOnce false :!label _label
    (:Completed
      (bind _alpha (Timeline|T_PressButton PlayFromStart)
        (:Update
          (Transformation|SetRelativeLocation (Variables|Default|GetButton) (Math|Vector|Lerp(Vector) "0.000000,0.000000,13.000000" "0.000000,0.000000,9.000000" _alpha) false false))
        (:Finished
          (goto _label Reset))))))

(event EventTick
  (params (DeltaSeconds :type Float%20%28single-precision%29))
  (Utilities|FlowControl|Sequence
    (:then_0
      (if (Variables|/Game/FirstPerson/Blueprints/BP_FirstPersonCharacter.BP_FirstPersonCharacter_C|GetIsHoveringOverObject? (Variables|Default|GetPlayerREF))
        (CallFunction|StartGame)
        (bind _alpha (Timeline|T_OpenCover Play)
          (:Update
            (Transformation|SetRelativeRotation (Variables|Default|GetCover) (Math|Rotator|Lerp(Rotator) "0, 0, 0" "105.000000,0.000000,0.000000" _alpha) false false)))
        (else
          (CallFunction|EndGame)
          (Timeline|T_OpenCover Reverse))))
    (:then_1
      (if (Variables|Default|GetWin?)
        (CallFunction|EndGame)
        (Rendering|Material|SetMaterial (Variables|Default|GetLight) 0 "/Game/Interactables/StaticMeshes/Materials/M_Yellow_Plastic.M_Yellow_Plastic")))))

(event EventBeginPlay
  (bind _asbp_first_person_character (Utilities|Casting|CastToBP_FirstPersonCharacter (Game|GetPlayerCharacter 0)))
  (Variables|Default|SetPlayerREF _asbp_first_person_character))

(fn ConstructionScript
  (|CallParentFunction))